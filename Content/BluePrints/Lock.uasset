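; Lock actor that is opened by touching it with a key, which removes both the lock and a key.
; On Box overlap with an actor tagged "Key", it destroys itself, plays the key-on-lock sound and calls DestroyKey.
; The sound location and DestroyKey target come from GetActorOfClass(Key), not from the overlapping actor.
; BeginPlay sets the lock's Tags from NewTag.
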(event OnComponentBeginOverlap(Box)
  (params (OverlappedComponent :type Primitive%20Component%20Object%20Reference) (OtherActor :type Actor%20Object%20Reference) (OtherComp :type Primitive%20Component%20Object%20Reference) (OtherBodyIndex :type Integer) (bFromSweep :type Boolean) (SweepResult :type Hit%20Result%20Structure%20%28by%20ref%29))
  (if (Actor|ActorHasTag OtherActor "Key")
    (CallFunction|DestroyLock)
    (bind _returnvalue (Actor|GetActorOfClass "/Game/BluePrints/Key.Key_C"))
    (Audio|PlaySoundatLocation "/Game/Sounds/Throw_KeyOnLock.Throw_KeyOnLock" (Transformation|GetActorLocation _returnvalue) "0, 0, 0" 1.0 1.0 0.0 0 0 0)
    (Default|DestroyKey _returnvalue)))

(event Custom|DestroyLock
  (Actor|DestroyActor))

(event EventBeginPlay
  (Variables|Default|SetTags (Variables|Default|GetNew%20Tag)))

(event EventTick
  (params (DeltaSeconds :type Float%20%28single-precision%29)))

(fn ConstructionScript)