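; Respawn Blueprint that records the starting transforms of level objects when play begins; the file contains no spawning logic itself.
; On BeginPlay it looks up one actor of each Key, Lock, Door, Heart, Water, Skull and Time variant class, storing each transform in its own variable.
; It also gathers every Fire actor into an array and appends their transforms to a parallel transform array.
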(event EventBeginPlay
  (bind _returnvalue (Actor|GetActorOfClass "/Game/BluePrints/Key.Key_C"))
  (Variables|Default|SetKeyTrans (Transformation|GetActorTransform _returnvalue))
  (bind _returnvalue_2 (Actor|GetActorOfClass "/Game/BluePrints/Time.Time_C"))
  (Variables|Default|SetTime1Trans (Transformation|GetActorTransform _returnvalue_2))
  (bind _returnvalue_3 (Actor|GetActorOfClass "/Game/BluePrints/Time_2.Time_2_C"))
  (Variables|Default|SetTime2Trans (Transformation|GetActorTransform _returnvalue_3))
  (bind _returnvalue_4 (Actor|GetActorOfClass "/Game/BluePrints/Time_3.Time_3_C"))
  (Variables|Default|SetTime3Trans (Transformation|GetActorTransform _returnvalue_4))
  (bind _returnvalue_5 (Actor|GetActorOfClass "/Game/BluePrints/Time_4.Time_4_C"))
  (Variables|Default|SetTime4Trans (Transformation|GetActorTransform _returnvalue_5))
  (bind _returnvalue_6 (Actor|GetActorOfClass "/Game/BluePrints/Lock.Lock_C"))
  (Variables|Default|SetLockTrans (Transformation|GetActorTransform _returnvalue_6))
  (bind _returnvalue_7 (Actor|GetActorOfClass "/Game/BluePrints/Heart.Heart_C"))
  (Variables|Default|SetHeartTrans (Transformation|GetActorTransform _returnvalue_7))
  (bind _returnvalue_8 (Actor|GetActorOfClass "/Game/BluePrints/Water.Water_C"))
  (Variables|Default|SetWaterTrans (Transformation|GetActorTransform _returnvalue_8))
  (bind _returnvalue_9 (Actor|GetActorOfClass "/Game/BluePrints/Door.Door_C"))
  (Variables|Default|SetDoorTrans (Transformation|GetActorTransform _returnvalue_9))
  (bind _returnvalue_10 (Actor|GetActorOfClass "/Game/BluePrints/Skull.Skull_C"))
  (Variables|Default|SetSkullTrans (Transformation|GetActorTransform _returnvalue_10))
  (bind _outactors (Actor|GetAllActorsOfClass "/Game/BluePrints/Fire.Fire_C"))
  (bind _output_get (Variables|Default|SetFireArray _outactors))
  (for _array_element _output_get
    (Utilities|Array|Add (Variables|Default|GetFireTrans) (Transformation|GetActorTransform _array_element))))

(fn ConstructionScript)