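; PC_Character runs a countdown that ends the player's control when time runs out, and creates the on-screen UI at BeginPlay.
; Tick lowers TimeRemaining roughly once a second through a Delay and loops a ticking sound gated by the PlaySound flag.
; Once the time drops below zero, it disables input on the player character, plays the time-out sound once and clears the flag.
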(event Custom|TickingSound
  (if (Variables|Default|GetPlaySound)
    (Variables|Default|SetPlaySound false)
    (Audio|PlaySound2D "/Game/Sounds/Time_Ticking.Time_Ticking" 1.0 1.0 0.0 0 0)
    (Utilities|FlowControl|Delay 5.25)
    (Variables|Default|SetPlaySound true)))

(event EventTick
  (params (DeltaSeconds :type Float%20%28single-precision%29))
  (CallFunction|TickingSound)
  (if (>= (Variables|Default|GetTimeRemaining) 0)
    (Utilities|FlowControl|Delay 1.0)
    (Math|Integer|DecrementInt (Variables|Default|GetTimeRemaining))
    (else
      (bind _ascharacter (Utilities|Casting|CastToCharacter (Game|Player|GetPlayerPawn 0)))
      (Input|DisableInput _ascharacter 0)
      (Utilities|FlowControl|DoOnce false
        (:Completed
          (Audio|PlaySound2D "/Game/Sounds/Time_Runs_Out.Time_Runs_Out" 1.0 1.0 0.0 0 0)
          (Variables|Default|SetPlaySound false))))))

(event EventBeginPlay
  (bind _returnvalue (UserInterface|CreateWidget "/Game/UI/UI.UI_C"))
  (UserInterface|Viewport|AddtoViewport _returnvalue 0))

(fn ConstructionScript)